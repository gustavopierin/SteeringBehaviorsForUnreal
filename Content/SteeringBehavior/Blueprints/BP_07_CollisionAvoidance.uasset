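; Steering-behavior actor that moves toward target actors while turning away from nearby obstacles, with its mesh added at construction.
; BeginPlay gathers targets and obstacles by class.
; Each Tick, Seek moves it forward, slows or stops it by distance and turns it toward the closest target, then Flee rotates it away from obstacles within range using negated-vector look-at.
; An uncalled test function draws eight-direction line traces.
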(event `self.ReceiveBeginPlay`
  (for _array_element (`self.Target`)
    (bind _outactors (`GameplayStatics.GetAllActorsOfClass` _array_element))
    (for _array_element_2 _outactors
      (`KismetArrayLibrary.Array_Add` (`self.ArrivalTarget`) _array_element_2)
      (for _array_element_3 (`self.Obstacles`)
        (bind _outactors_2 (`GameplayStatics.GetAllActorsOfClass` _array_element_3))
        (for _array_element_4 _outactors_2
          (`KismetArrayLibrary.Array_Add` (`self.FleeTarget`) _array_element_4))))))

(event `self.ReceiveTick`
  (params (DeltaSeconds :type "Float (single-precision)"))
  (`|ExecutionSequence`
    (:`then_0`
      (`self.Seek`))
    (:`then_1`
      (`self.Flee`))))

(fn `Flee`
  (if (`self.MultiplesObstacles`)
    (for (_ _array_index) (`self.FleeTarget`)
      ;[1 1 1] Defines a minimum distance between Static Mesh and Target
      (if (< (`self.GetDistanceTo` (`|GetArrayItem` (`self.FleeTarget`) _array_index)) (`self.AvoidanceDistance`)) :!label _label
        (`self.K2_SetActorRotation` (`KismetMathLibrary.RInterpTo` (`self.K2_GetActorRotation`) (`KismetMathLibrary.FindLookAtRotation` (`KismetMathLibrary.NegateVector` (`self.K2_GetActorLocation`)) (`KismetMathLibrary.NegateVector` (`self.K2_GetActorLocation` (`|GetArrayItem` (`self.FleeTarget`) _array_index)))) (`GameplayStatics.GetWorldDeltaSeconds`) 3.0))))
    (else
      (goto _label))))

(fn `Seek`
  (`|ExecutionSequence`
    (:`then_0`
      ;[1 1 1] This sets the Static Mesh to move 5 units forward
      (`self.K2_AddActorLocalOffset` (`KismetMathLibrary.MakeVector` (`self.Velocity`))))
    (:`then_1`
      (if (`self.ClosestTarget`)
        (for (_array_element _array_index) (`self.ArrivalTarget`)
          (bind _returnvalue (`self.GetDistanceTo` _array_element))
          ;[1 1 1] Stores the distances between the Actor and the Targets
          (`KismetArrayLibrary.Array_Set` (`self.TargetDistance`) _array_index _returnvalue true)
          ;[1 1 1] Set a minimum distance between the Static Mesh and the Target to initiate a deceleration
          (if (> _returnvalue (`self.DecelerationMinimumDistance`)) :!label _label
            _
            (elif (> _returnvalue (`self.StopMinimumDistance`))
              (set `self.Velocity` (/ _returnvalue (`self.DecelerationIntensity`)))
              (else
                (set `self.Velocity` 0.0))))
          ;[1 1 1] Set the Static Mesh to rotate based on the Target's location
          (`self.K2_SetActorRotation` (`KismetMathLibrary.RInterpTo` (`self.K2_GetActorRotation`) (`KismetMathLibrary.FindLookAtRotation` (`self.K2_GetActorLocation`) (`self.K2_GetActorLocation` (`|GetArrayItem` (`self.ArrivalTarget`) (`KismetMathLibrary.MinOfFloatArray` (`self.TargetDistance`))))) (`GameplayStatics.GetWorldDeltaSeconds`) 5.0)))
        (else
          (goto _label))))))

(fn `TraceAvoidance(Test)`
  (bind _returnvalue (`self.K2_GetActorLocation`))
  ;[1 1 1] Isso cria o LineTrace
  (for _index (range 8)
    (`KismetSystemLibrary.LineTraceSingle` :`Start` _returnvalue :`End` (+ _returnvalue (select `int` _index :`0` (0.0 300.0 0.0) :`1` (0.0 -300.0 0.0) :`2` (300.0 0.0 0.0) :`3` (-300.0 0.0 0.0) :`4` (200.0 -200.0 0.0) :`5` (-200.0 200.0 0.0) :`6` (-200.0 -200.0 0.0) :`7` (200.0 200.0 0.0) :!type "Vector Structure")) :`TraceChannel` "TraceTypeQuery1" :`DrawDebugType` "ForOneFrame")))

(fn `UserConstructionScript`
  (bind _returnvalue (`AddComponent|NODE_AddStaticMeshComponent-0` :`RelativeTransform` (`KismetMathLibrary.MakeTransform` (0.0 0.0 -50.0))))
  (`StaticMeshComponent.SetStaticMesh` _returnvalue (`self.StaticMesh`)))