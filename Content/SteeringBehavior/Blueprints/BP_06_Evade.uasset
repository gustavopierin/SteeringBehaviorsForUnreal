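; BP_06_Evade is a steering-behavior actor that constantly moves forward and turns away from where its targets are heading.
; BeginPlay gathers all actors of the EvadeTarget classes, and construction adds its static mesh.
; On Tick, within a minimum distance of a point projected ahead of a target, it smoothly rotates away using a look-at between negated positions.
; MultipleTarget checks every target; otherwise a single check reuses the loop's index.
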(event `self.ReceiveBeginPlay`
  (for _array_element (`self.EvadeTarget`)
    (bind _outactors (`GameplayStatics.GetAllActorsOfClass` _array_element))
    (for _array_element_2 _outactors
      (`KismetArrayLibrary.Array_Add` (`self.Target`) _array_element_2))))

(event `self.ReceiveTick`
  (params (DeltaSeconds :type "Float (single-precision)"))
  (`|ExecutionSequence`
    (:`then_0`
      ;[1 1 1] This sets the Static Mesh to move 5 units forward
      (`self.K2_AddActorLocalOffset` (`KismetMathLibrary.MakeVector` (`self.Velocity`))))
    (:`then_1`
      (if (`self.MultipleTarget`)
        (for (_ _array_index) (`self.Target`)
          (bind _output (`|GetArrayItem` (`self.Target`) _array_index))
          ;[1 1 1] Defines a minimum distance between Static Mesh and Target + 500 units forward
          (if (< (`KismetMathLibrary.Vector_Distance` (`self.K2_GetActorLocation`) (+ (`self.K2_GetActorLocation` _output) (* (`self.GetActorForwardVector` _output) (`self.TargetForwardDistance`)))) (`self.EffectMinimumDistance`)) :!label _label
            (bind _output_2 (`|GetArrayItem` (`self.Target`) _array_index))
            ;[1 1 1] This sets the Static Mesh to rotate based on the opposite location of Target + 500 units in front
            (`self.K2_SetActorRotation` (`KismetMathLibrary.RInterpTo` (`self.K2_GetActorRotation`) (`KismetMathLibrary.FindLookAtRotation` (`KismetMathLibrary.NegateVector` (`self.K2_GetActorLocation`)) (`KismetMathLibrary.NegateVector` (+ (`self.K2_GetActorLocation` _output_2) (* (`self.GetActorForwardVector` _output_2) (`self.TargetForwardDistance`))))) (`GameplayStatics.GetWorldDeltaSeconds`) 5.0))))
        (else
          (goto _label))))))

(fn `UserConstructionScript`
  (bind _returnvalue (`AddComponent|NODE_AddStaticMeshComponent-0` :`RelativeTransform` (`KismetMathLibrary.MakeTransform` (0.0 0.0 -50.0))))
  (`StaticMeshComponent.SetStaticMesh` _returnvalue (`self.StaticMesh`)))