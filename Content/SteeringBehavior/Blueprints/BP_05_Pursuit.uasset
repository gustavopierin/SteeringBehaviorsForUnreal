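; Steering-behavior pursuit actor that chases a point projected ahead of the nearest actor of its target classes.
; BeginPlay gathers the targets; each Tick moves it along local X by Velocity, without delta-time scaling, and smoothly turns it toward that predicted point.
; With ClosestTarget set, it records distances and applies distance-based slowing and stopping per target, so the last one evaluated sets Velocity.
; The construction script adds its mesh.
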(event `self.ReceiveBeginPlay`
  (for _array_element (`self.Target`)
    (bind _outactors (`GameplayStatics.GetAllActorsOfClass` _array_element))
    (for _array_element_2 _outactors
      (`KismetArrayLibrary.Array_Add` (`self.PursuitTarget`) _array_element_2))))

(event `self.ReceiveTick`
  (params (DeltaSeconds :type "Float (single-precision)"))
  (bind _output (`|GetArrayItem` (`self.PursuitTarget`) (`KismetMathLibrary.MinOfFloatArray` (`self.TargetDistance`))))
  (`|ExecutionSequence`
    (:`then_0`
      ;[1 1 1] This sets the Static Mesh to move 5 units forward
      (`self.K2_AddActorLocalOffset` (`KismetMathLibrary.MakeVector` (`self.Velocity`))))
    (:`then_1`
      (if (`self.ClosestTarget`)
        (for (_array_element _array_index) (`self.PursuitTarget`)
          (bind _returnvalue (`self.GetDistanceTo` _array_element))
          ;[1 1 1] Stores the distances between the Actor and the Targets
          (`KismetArrayLibrary.Array_Set` (`self.TargetDistance`) _array_index _returnvalue true)
          ;[1 1 1] Set a minimum distance between the Static Mesh and the Target to initiate a deceleration
          (if (> _returnvalue (`self.DecelerationMinimumDistance`)) :!label _label
            (set `self.Velocity` (`self.Velocity`))
            (elif (> _returnvalue (`self.StopMinimumDistance`))
              (set `self.Velocity` (/ _returnvalue (`self.DecelerationIntensity`)))
              (else
                (set `self.Velocity` 0.0)))))
        (else
          (goto _label))))
    (:`then_2`
      ;[1 1 1] This sets the Static Mesh to rotate based on the location of the Target + 500 units in the front(ForwardDistance)
      (`self.K2_SetActorRotation` (`KismetMathLibrary.RInterpTo` (`self.K2_GetActorRotation`) (`KismetMathLibrary.FindLookAtRotation` (`self.K2_GetActorLocation`) (+ (`self.K2_GetActorLocation` _output) (* (`self.GetActorForwardVector` _output) (`self.TargetForwardDistance`)))) (`GameplayStatics.GetWorldDeltaSeconds`) 5.0)))))

(fn `UserConstructionScript`
  (bind _returnvalue (`AddComponent|NODE_AddStaticMeshComponent-0` :`RelativeTransform` (`KismetMathLibrary.MakeTransform` (0.0 0.0 -50.0))))
  (`StaticMeshComponent.SetStaticMesh` _returnvalue (`self.StaticMesh`)))