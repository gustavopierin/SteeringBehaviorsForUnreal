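; Flocking actor that spawns a number of static mesh components and moves them as a steering-behavior flock.
; Each Tick moves every mesh forward and turns it toward a random point around a pivot, or around the actor when the pivot strays beyond the flock radius.
; Every two seconds the pivot jumps to a random member, with new turn speed and vertical bias.
; Optional avoidance compares all pairs, turning meshes away from close neighbors.
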(event `self.ReceiveBeginPlay`
  ;[1 1 1] Add an N amount of Static mesh
  (for _ (range 1 (+ (`self.NumberOfFlock`) 1))
    ;[1 1 1] Set a Static Mesh
    (bind _returnvalue (`AddComponent|NODE_AddStaticMeshComponent-0`))
    (`StaticMeshComponent.SetStaticMesh` _returnvalue (`self.StaticMesh`))
    ;[1 1 1] Add the Static Mesh in 2 arrays (one for avoidance verification)
    (`KismetArrayLibrary.Array_Add` (`self.Flock`) _returnvalue)
    (`KismetArrayLibrary.Array_Add` (`self.FlockFlee`) _returnvalue))
  ;[1 1 1] Set a Turn Speed when Actor play.
  (`self.UpdateTurnSpeed`))

(event `UpdateFlockPivot`
  ;[1 1 1] Randomly chooses a Static Mesh to be the pivot
  (set `self.FlockPivot` (`SceneComponent.K2_GetComponentLocation` (`|GetArrayItem` (`self.Flock`) (`KismetMathLibrary.RandomInteger` (`self.NumberOfFlock`))))))

(event `UpdateTurnSpeed`
  ;[1 1 1] Randomly change the Turn Speed value
  (set `self.TurnSpeed` (`KismetMathLibrary.RandomFloatInRange` 0.05 2.0)))

(event `self.ReceiveTick`
  (params (DeltaSeconds :type "Float (single-precision)"))
  (`|ExecutionSequence`
    (:`then_0`
      ;[1 1 1] Every 2 sec updates the pivot, turn speed and height
      (`KismetSystemLibrary.Delay` 2.0)
      (`self.UpdateFlockPivot`)
      (`self.UpdateTurnSpeed`)
      (set `self.CimaBaixoOuNenhum` (`KismetMathLibrary.RandomInteger` 3)))
    (:`then_1`
      ;[1 1 1] All this runs for each Static Mesh
      (for (_array_element _array_index) (`self.Flock`)
        (set `self.FlockElement` _array_element)
        (set `self.FlockIndex` _array_index)
        (`|ExecutionSequence`
          (:`then_0`
            (`self.Flocking Velocity`))
          (:`then_1`
            (`self.Rotation`))
          (:`then_2`
            (`self.NewDestination`))
          (:`then_3`
            (`self.Flee`)))))))

(fn `Flee`
  (bind _flockelement (`self.FlockElement`))
  ;[1 1 1] Turn Avoidance On or Off
  (if (`self.TurnAvoidanceOn`)
    ;[1 1 1] Remove the current Static Mesh from the Flock Flee array
    (`KismetArrayLibrary.Array_RemoveItem` (`self.FlockFlee`) (`self.FlockElement`))
    (for _array_element (`self.FlockFlee`)
      (set `self.FlockElementLessOne` _array_element)
      ;[1 1 1] Compare the distance of each element of the Flock Flee array with the current Flock Element
      (if (< (`KismetMathLibrary.Vector_Distance` (`SceneComponent.K2_GetComponentLocation` (`self.FlockElement`)) (`SceneComponent.K2_GetComponentLocation` (`self.FlockElementLessOne`))) (`self.AvoidanceDistance`))
        ;[1 1 1] Distance the staic mesh from the other staic meshes
        (`SceneComponent.K2_SetWorldRotation` _flockelement (`KismetMathLibrary.RInterpTo` (`SceneComponent.K2_GetComponentRotation` _flockelement) (`KismetMathLibrary.FindLookAtRotation` (`KismetMathLibrary.NegateVector` (`SceneComponent.K2_GetComponentLocation` _flockelement)) (`KismetMathLibrary.NegateVector` (`SceneComponent.K2_GetComponentLocation` (`self.FlockElementLessOne`)))) (`GameplayStatics.GetWorldDeltaSeconds`) 5.0) false false)))
    ;[1 1 1] At the end of the comparison add again the current element in the Flock Flee array
    (`KismetArrayLibrary.Array_Add` (`self.FlockFlee`) (`self.FlockElement`))))

(fn `Flocking Velocity`
  ;[1 1 1] This moves each Static Mesh forward
  (`SceneComponent.K2_AddLocalOffset` (`self.FlockElement`) (`KismetMathLibrary.MakeVector` (`self.Velocity`)) false false))

(fn `NewDestination`
  (bind _maximumtravelspace (`self.MaximumTravelSpace`))
  ;[1 1 1] Set a random point to be the new direction
  (set `self.NDestination` (`KismetMathLibrary.RandomPointInBoundingBox` (select `bool` (> (`KismetMathLibrary.Vector_Distance` (`self.FlockPivot`) (`self.K2_GetActorLocation`)) (`self.FlockingSize`)) :`false` (+ (`self.FlockPivot`) (select `int` (`self.CimaBaixoOuNenhum`) :`0` (0.0 0.0 1000.0) :`1` (0.0 0.0 -1000.0) :`2` (0.0 0.0 0.0) :!type "Vector Structure")) :`true` (`self.K2_GetActorLocation`)) (`KismetMathLibrary.MakeVector` _maximumtravelspace _maximumtravelspace _maximumtravelspace)))
  ;[1 1 1] a New Direction no array Flock Destination
  (`KismetArrayLibrary.Array_Set` (`self.FlockDestinations`) (`self.FlockIndex`) (`self.NDestination`) true))

(fn `Rotation`
  (bind _flockelement (`self.FlockElement`))
  ;[1 1 1] Rotates each Static Mesh to a new location
  (`SceneComponent.K2_SetWorldRotation` _flockelement (`KismetMathLibrary.RInterpTo` (`SceneComponent.K2_GetComponentRotation` _flockelement) (`KismetMathLibrary.FindLookAtRotation` (`SceneComponent.K2_GetComponentLocation` _flockelement) (`|GetArrayItem` (`self.FlockDestinations`) (`self.FlockIndex`))) (`GameplayStatics.GetWorldDeltaSeconds`) (`self.TurnSpeed`)) false false))

(fn `UserConstructionScript`
  (`SphereComponent.SetSphereRadius` (`self.Sphere`) (`self.FlockingSize`) false))