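; Steering-behavior actor that follows a list of path points, optionally starting at the closest one, with its static mesh added at construction.
; Each tick it moves along its local forward axis while smoothly rotating toward the current point.
; Speed scales down with distance inside a deceleration radius and drops to zero inside a stop radius.
; On reaching a point it waits, then advances, either looping or ping-ponging along the path.
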(event `self.ReceiveBeginPlay`
  ;[1 1 1] Chose the closest path point
  (if (`self.ClosestPath`)
    (for (_array_element _array_index) (`self.PathPoints`)
      (`KismetArrayLibrary.Array_Set` (`self.AllPathDistance`) _array_index (`KismetMathLibrary.Vector_Distance` (`self.K2_GetActorLocation`) _array_element) true)
      (set `self.PathIndex` (`KismetMathLibrary.MinOfFloatArray` (`self.AllPathDistance`))))))

(event `self.ReceiveTick`
  (params (DeltaSeconds :type "Float (single-precision)"))
  (bind _returnvalue (`KismetMathLibrary.Vector_Distance` (`self.K2_GetActorLocation`) (`|GetArrayItem` (`self.PathPoints`) (`self.PathIndex`))))
  (`|ExecutionSequence`
    (:`then_0`
      ;[1 1 1] Actor Velocity
      (`self.K2_AddActorLocalOffset` (`KismetMathLibrary.MakeVector` (`self.Velocity`))))
    (:`then_1`
      ;[1 1 1] Actor Direction
      (`self.K2_SetActorRotation` (`KismetMathLibrary.RInterpTo` (`self.K2_GetActorRotation`) (`KismetMathLibrary.FindLookAtRotation` (`self.K2_GetActorLocation`) (`|GetArrayItem` (`self.PathPoints`) (`self.PathIndex`))) (`GameplayStatics.GetWorldDeltaSeconds`) 5.0)))
    (:`then_2`
      ;[1 1 1] Comment
      (for (_array_element _array_index) (`self.PathPoints`)
        (`KismetArrayLibrary.Array_Set` (`self.AllPathDistance`) _array_index (`KismetMathLibrary.Vector_Distance` (`self.K2_GetActorLocation`) _array_element) true)))
    (:`then_3`
      ;[1 1 1] Actor Deceleration
      (set `self.PathDistance` _returnvalue)
      (if (> _returnvalue (`self.DecelerationMinimumDistance`))
        (set `self.Velocity` 7.0)
        (elif (> _returnvalue (`self.StopMinimumDistance`))
          (set `self.Velocity` (/ _returnvalue (`self.DecelerationIntensity`)))
          (else
            (set `self.Velocity` 0.0)))))
    (:`then_4`
      (if (`self.Loop`)
        ;[1 1 1] Loop
        (if (== (`self.K2_GetActorLocation`) (`|GetArrayItem` (`self.PathPoints`) (`self.PathIndex`)) :`ErrorTolerance` 100.0)
          (`KismetSystemLibrary.Delay` (`self.WaitTime`))
          (`/Engine/EditorBlueprintResources/StandardMacros.IncrementInt` (`self.PathIndex`)
            (:`  `
              (if (>= (`self.PathIndex`) (`KismetArrayLibrary.Array_Length` (`self.PathPoints`)))
                (set `self.PathIndex` 0)))))
        (else
          ;[1 1 1] --->  <---
          (if (== (`self.K2_GetActorLocation`) (`|GetArrayItem` (`self.PathPoints`) (`self.PathIndex`)) :`ErrorTolerance` 100.0)
            (if (`self.IncrementOrDecrement`)
              (`KismetSystemLibrary.Delay` (`self.WaitTime`))
              (if (<= (+ (`self.PathIndex`) 1) (- (`KismetArrayLibrary.Array_Length` (`self.PathPoints`)) 1))
                (`/Engine/EditorBlueprintResources/StandardMacros.IncrementInt` (`self.PathIndex`))
                (else
                  (set `self.IncrementOrDecrement` false)))
              (else
                (`KismetSystemLibrary.Delay` (`self.WaitTime`))
                (if (>= (`self.PathIndex`) 1)
                  (`/Engine/EditorBlueprintResources/StandardMacros.DecrementInt` (`self.PathIndex`))
                  (else
                    (set `self.IncrementOrDecrement` true)))))))))))

(fn `UserConstructionScript`
  (bind _returnvalue (`AddComponent|NODE_AddStaticMeshComponent-0` :`RelativeTransform` (`KismetMathLibrary.MakeTransform` (0.0 0.0 -50.0))))
  (`StaticMeshComponent.SetStaticMesh` _returnvalue (`self.StaticMesh`)))