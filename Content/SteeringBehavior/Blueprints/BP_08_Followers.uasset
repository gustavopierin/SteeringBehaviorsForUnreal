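; Follower actor for a leader-following steering demo, moving forward each Tick and steered by Arrival, Evade and Flee.
; BeginPlay collects leaders and avoidance actors from configurable class arrays.
; Arrival slows or stops it near leaders and can turn it toward the nearest.
; Evade turns it away from points ahead of leaders, and Flee from nearby avoidance actors, using interpolated look-at rotations on negated positions.
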(event `self.ReceiveBeginPlay`
  (for _array_element (`self.Target`)
    (bind _outactors (`GameplayStatics.GetAllActorsOfClass` _array_element))
    (for _array_element_2 _outactors
      (`KismetArrayLibrary.Array_Add` (`self.ArrivalEvadeTarget`) _array_element_2)
      (for _array_element_3 (`self.AvoidanceTarget`)
        (bind _outactors_2 (`GameplayStatics.GetAllActorsOfClass` _array_element_3))
        (for _array_element_4 _outactors_2
          (`KismetArrayLibrary.Array_Add` (`self.FleeTarget`) _array_element_4))))))

(event `self.ReceiveTick`
  (params (DeltaSeconds :type "Float (single-precision)"))
  (`|ExecutionSequence`
    (:`then_0`
      (`self.Arrival`))
    (:`then_1`
      (`self.Evade`))
    (:`then_2`
      (`self.Flee`))))

(fn `Arrival`
  (`|ExecutionSequence`
    (:`then_0`
      ;[1 1 1] This sets the Static Mesh to move 5 units forward
      (`self.K2_AddActorLocalOffset` (`KismetMathLibrary.MakeVector` (`self.Velocity`))))
    (:`then_1`
      (if (`self.ClosestTarget`)
        (for (_array_element _array_index) (`self.ArrivalEvadeTarget`)
          (bind _returnvalue (`self.GetDistanceTo` _array_element))
          ;[1 1 1] Stores the distances between the Actor and the Targets
          (`KismetArrayLibrary.Array_Set` (`self.LeaderDistance`) _array_index _returnvalue true)
          ;[1 1 1] Set a minimum distance between the Static Mesh and the Target to initiate a deceleration
          (if (>= _returnvalue (`self.DecelerationMinimumDistance`)) :!label _label
            _
            (elif (>= _returnvalue (`self.StopMinimumDistance`))
              (set `self.Velocity` (/ _returnvalue (`self.DecelerationIntensity`)))
              (else
                (set `self.Velocity` 0.0))))
          ;[1 1 1] Set the Static Mesh to rotate based on the Target's location
          (`self.K2_SetActorRotation` (`KismetMathLibrary.RInterpTo` (`self.K2_GetActorRotation`) (`KismetMathLibrary.FindLookAtRotation` (`self.K2_GetActorLocation`) (`self.K2_GetActorLocation` (`|GetArrayItem` (`self.ArrivalEvadeTarget`) (`KismetMathLibrary.MinOfFloatArray` (`self.LeaderDistance`))))) (`GameplayStatics.GetWorldDeltaSeconds`) 5.0)))
        (else
          (goto _label))))))

(fn `Evade`
  (if (`self.MultipleTarget`)
    (for (_ _array_index) (`self.ArrivalEvadeTarget`)
      (bind _output (`|GetArrayItem` (`self.ArrivalEvadeTarget`) _array_index))
      ;[1 1 1] Defines a minimum distance between Static Mesh and Target + 500 units forward
      (if (< (`KismetMathLibrary.Vector_Distance` (`self.K2_GetActorLocation`) (+ (`self.K2_GetActorLocation` _output) (* (`self.GetActorForwardVector` _output) (`self.ForwardDistance`)))) (`self.EffectMinimumDistance`)) :!label _label
        (bind _output_2 (`|GetArrayItem` (`self.ArrivalEvadeTarget`) _array_index))
        ;[1 1 1] This sets the Static Mesh to rotate based on the opposite location of Target + 500 units in front
        (`self.K2_SetActorRotation` (`KismetMathLibrary.RInterpTo` (`self.K2_GetActorRotation`) (`KismetMathLibrary.FindLookAtRotation` (`KismetMathLibrary.NegateVector` (`self.K2_GetActorLocation`)) (`KismetMathLibrary.NegateVector` (+ (`self.K2_GetActorLocation` _output_2) (* (`self.GetActorForwardVector` _output_2) (`self.ForwardDistance`))))) (`GameplayStatics.GetWorldDeltaSeconds`) 5.0))))
    (else
      (goto _label))))

(fn `Flee`
  (for _array_element (`self.FleeTarget`)
    ;[1 1 1] Removes the current element so that it does not apply Flee Efect to itself
    (`KismetArrayLibrary.Array_RemoveItem` (`self.FleeTarget`) self)
    ;[1 1 1] Defines a minimum distance between Static Mesh and Target
    (if (< (`self.GetDistanceTo` _array_element) (`self.AvoidanceDistance`))
      ;[1 1 1] Set the Static Mesh to rotate based on the target's opposite location
      (`self.K2_SetActorRotation` (`KismetMathLibrary.RInterpTo` (`self.K2_GetActorRotation`) (`KismetMathLibrary.FindLookAtRotation` (`KismetMathLibrary.NegateVector` (`self.K2_GetActorLocation`)) (`KismetMathLibrary.NegateVector` (`self.K2_GetActorLocation` _array_element))) (`GameplayStatics.GetWorldDeltaSeconds`) 3.0))))
  ;[1 1 1] At the end of the current loop add the element again
  (`KismetArrayLibrary.Array_Add` (`self.FleeTarget`) self))

(fn `UserConstructionScript`
  (bind _returnvalue (`AddComponent|NODE_AddStaticMeshComponent-0` :`RelativeTransform` (`KismetMathLibrary.MakeTransform` (0.0 0.0 -50.0))))
  (`StaticMeshComponent.SetStaticMesh` _returnvalue (`self.StaticMesh`)))